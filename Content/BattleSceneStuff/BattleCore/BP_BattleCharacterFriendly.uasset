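; BP_BattleCharacterFriendly is a battle character Blueprint for friendly combatants, handling their timer-based attack readiness.
; AttackReady pauses the CombatTimer and sets CanAttack, holding the character in a ready state.
; ResetTimer, only when CanAttack is set, clears and invalidates that timer and calls StartAttacking.
; The construction script only calls its parent.
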(event Custom|ResetTimer
  (if (Variables|Default|GetCanAttack)
    (Utilities|Time|ClearandInvalidateTimerbyHandle (Variables|Default|GetCombatTimer))
    (CallFunction|StartAttacking)))

(event EventAttackReady
  (Utilities|Time|PauseTimerbyHandle (Variables|Default|GetCombatTimer))
  (Variables|Default|SetCanAttack true))

(fn ConstructionScript
  (|CallParentFunction))