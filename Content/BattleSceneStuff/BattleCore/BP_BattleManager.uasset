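; Battle manager that loads the area's battle scene as an offset level instance and sets up party-versus-enemy combat.
; After loading, it gathers spawn points and the battle camera from that level.
; StartBattle disables player movement, shows the combat HUD, spawns both sides facing each other, fills the party UI and blends to the camera.
; GetTurnOrder sorts combatants by randomized, Speed-weighted keys, though nothing here calls it.
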(event Custom|Set%20Battle%20Scene
  ;[0.15 0.15 0.15 0.5] Load
  (Utilities|FlowControl|Sequence
    (:then_0
      (bind _outactors (Actor|GetAllActorsOfClass "/Game/BattleSceneStuff/Spawns/BP_BSPFriendly.BP_BSPFriendly_C"))
      (Variables|Spawns|SetFriendlySpawns _outactors))
    (:then_1
      (bind _returnvalue (Actor|GetActorOfClass "/Game/BattleSceneStuff/BattleCore/BP_BattleLevelManager.BP_BattleLevelManager_C"))
      (bind _output_get (Variables|Core|SetLevelBattleManager _returnvalue))
      (Variables|Core|SetBattleCamera (Variables|/Game/BattleSceneStuff/BattleCore/BP_BattleLevelManager.BP_BattleLevelManager_C|GetBattleCamera _output_get)))
    (:then_2
      (bind _outactors_2 (Actor|GetAllActorsOfClass "/Game/BattleSceneStuff/Spawns/BP_BSPEnemy.BP_BSPEnemy_C"))
      (Variables|Spawns|SetEnemySpawns _outactors_2))))

(event Custom|GetTurnOrder
  ;[0.15 0.15 0.15 0.5] TurnOrder
  (for _array_element (Variables|TurnTest|GetCharactersInCombat)
    (Utilities|Map|Add (Variables|TurnTest|GetSpeedMap) (+ (* (.speed (Variables|/Game/BattleSceneStuff/BattleCore/BP_BattleCharacter.BP_BattleCharacter_C|GetEnemyData _array_element)) 100) (Math|Random|RandomInteger 100)) _array_element))
  (bind _keys (Utilities|Map|Keys (Variables|TurnTest|GetSpeedMap)))
  (bind _output_get (Variables|TurnTest|SetSpeedValues _keys))
  (Class|KismetArrayLibrary|SortIntArray _output_get false "Descending")
  (for _array_element_2 (Variables|TurnTest|GetSpeedValues)
    (Utilities|Array|Add (Variables|TurnTest|GetTurnOrder) (.Value (Utilities|Map|Find (Variables|TurnTest|GetSpeedMap) _array_element_2)))))

(event Custom|EnemyLogic
  ;[0.15 0.15 0.15 0.5] Character Logic
  (for (_array_element _array_index) (Variables|Spawns|GetEnemySpawns)
    (bind _returnvalue (Game|SpawnActorfromClass :Class "/Game/BattleSceneStuff/BattleCore/BP_BattleCharacterEnemy.BP_BattleCharacterEnemy_C" :SpawnTransform (Math|Transform|MakeTransform (Transformation|GetActorLocation _array_element) (Math|Rotator|FindLookatRotation (Transformation|GetActorLocation _array_element) (Transformation|GetActorLocation (Utilities|Array|Get(acopy) (Variables|Spawns|GetFriendlySpawns) _array_index))) "1.000000,1.000000,1.000000") :CollisionHandlingOverride "Undefined" :TransformScaleMethod "MultiplyWithRoot" :RowName (.rowname (Utilities|Array|Get(acopy) (Variables|Default|GetEnemies) _array_index)) :BattleManager self :Instigator 0))
    (Utilities|Array|Add (Variables|TurnTest|GetCharactersInCombat) _returnvalue)))

(event Custom|FriendlyLogic
  ;[0.15 0.15 0.15 0.5] Character Logic
  (for (_array_element _array_index) (Variables|Spawns|GetFriendlySpawns)
    (bind _returnvalue (Game|SpawnActorfromClass "/Game/BattleSceneStuff/BattleCore/BP_BattleCharacterFriendly.BP_BattleCharacterFriendly_C" (Math|Transform|MakeTransform (Transformation|GetActorLocation _array_element) (Math|Rotator|MakeRotator 0.0 0.0 (.yaw (Math|Rotator|FindLookatRotation (Transformation|GetActorLocation _array_element) (Transformation|GetActorLocation (Utilities|Array|Get(acopy) (Variables|Spawns|GetEnemySpawns) _array_index))))) "1.000000,1.000000,1.000000") "Undefined" "MultiplyWithRoot" 0 (Utilities|Array|Get(acopy) (Variables|Core|GetTestParty) _array_index) "" self 0))
    (Utilities|Array|Add (Variables|TurnTest|GetCharactersInCombat) _returnvalue)
    (Utilities|Array|Add (Variables|Default|GetPlayerParty) _returnvalue))
  (CallFunction|BattleUI))

(event Custom|BattleUI
  (bind _playercontroller (Variables|Core|GetPlayerController))
  (bind _combathud (Variables|/Game/ThirdPerson/Blueprints/BP_ThirdPersonPlayerController.BP_ThirdPersonPlayerController_C|GetCombatHUD _playercontroller))
  (Variables|/Game/BattleSceneStuff/UI/WBP_CombatUI.WBP_CombatUI_C|SetPlayerParty _combathud (Variables|Default|GetPlayerParty))
  (Default|PopulateUI _combathud))

(event Custom|Start%20Battle
  (params (Enemies :type Array%20of%20Data%20Table%20Row%20Handle%20Structures))
  ;[0.15 0.15 0.15 0.5] Start
  (Variables|Default|SetEnemies Enemies)
  (Components|Activation|SetActive (Pawn|GetMovementComponent (Game|Player|GetPlayerPawn 0)) false false)
  ;;[0.15 0.15 0.15 0.5] PlayCutscene
  (Default|ShowCombatHud (Variables|Core|GetPlayerController))
  (Variables|/Script/Engine.PlayerController|SetbShowMouseCursor (Variables|Core|GetPlayerController) true)
  (CallFunction|FriendlyLogic)
  (CallFunction|EnemyLogic)
  (Utilities|FlowControl|Delay 1.25)
  (Game|Player|SetViewTargetwithBlend (Game|GetPlayerController 0) (Variables|Core|GetBattleCamera) 0.0 "VTBlend_Linear" 0.0 false))

(event Custom|Load%20Current%20Area%20Battle%20Scene
  ;[0.15 0.15 0.15 0.5] Init
  (Utilities|FlowControl|Sequence
    (:then_0
      (bind _returnvalue (Class|LevelStreamingDynamic|LoadLevelInstancebySoftObjectPtr (Variables|Default|GetAreaBattleScene) "5000.000000,5000.000000,0.000000" "0, 0, 0" "" 0 false))
      (Variables|Core|SetBattleInstance _returnvalue)
      (Utilities|FlowControl|Delay 0.25)
      (CallFunction|SetBattleScene))
    (:then_1
      (bind _asbp_third_person_player_controller (Utilities|Casting|CastToBP_ThirdPersonPlayerController (Game|GetPlayerController 0)))
      (Variables|Core|SetPlayerController _asbp_third_person_player_controller))))

(event EventBeginPlay
  ;[0.15 0.15 0.15 0.5] Init
  (Utilities|FlowControl|Sequence
    (:then_0
      (bind _returnvalue (Class|LevelStreamingDynamic|LoadLevelInstancebySoftObjectPtr (Variables|Default|GetAreaBattleScene) "5000.000000,5000.000000,0.000000" "0, 0, 0" "" 0 false))
      (Variables|Core|SetBattleInstance _returnvalue)
      (Utilities|FlowControl|Delay 0.25)
      (CallFunction|SetBattleScene))
    (:then_1
      (bind _asbp_third_person_player_controller (Utilities|Casting|CastToBP_ThirdPersonPlayerController (Game|GetPlayerController 0)))
      (Variables|Core|SetPlayerController _asbp_third_person_player_controller))))

(fn ConstructionScript)